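; Chicken livestock building Blueprint, a child that leaves its behavior to the parent class.
; On BeginPlay it runs the parent logic, then fills BuildingParts with its mesh components: cubes, modular wooden roofs, gables, beams and broken wooden pieces.
; The construction script only calls the parent, and the overlap and tick events are disabled.
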(event `self.ReceiveBeginPlay`
  (`parent.ReceiveBeginPlay`)
  (set `self.BuildingParts` (`|MakeArray` (`self.Cube`) (`self.Cube1`) (`self.Cube2`) (`self.Cube3`) (`self.S_Modular_Wooden_Roof_wkupbctdw_lod3_Var4`) (`self.S_Medieval_Gable_ueojafodw_lod3_Var2`) (`self.S_Modular_Wooden_Roof_wkupbctdw_lod3_Var2`) (`self.S_Modular_Wooden_Roof_wkupbctdw_lod3_Var3`) (`self.S_Medieval_Gable_ueojafodw_lod3_Var1`) (`self.Cube4`) (`self.S_Wooden_Beam_tgnheinfa_lod4`) (`self.S_Wooden_Beam_tgnheinfa_lod3`) (`self.S_Broken_Wooden_Piece_tjuiagajw_lod14`) (`self.S_Broken_Wooden_Piece_tjuiagajw_lod13`) (`self.S_Broken_Wooden_Piece_tjuiagajw_lod12`) (`self.S_Broken_Wooden_Piece_tjuiagajw_lod11`) (`self.S_Broken_Wooden_Piece_tjuiagajw_lod9`) (`self.S_Broken_Wooden_Piece_tjuiagajw_lod10`) (`self.S_Broken_Wooden_Piece_tjuiagajw_lod8`) (`self.S_Broken_Wooden_Piece_tjuiagajw_lod7`) (`self.S_Broken_Wooden_Piece_tjuiagajw_lod6`) (`self.S_Broken_Wooden_Piece_tjuiagajw_lod5`) (`self.S_Broken_Wooden_Piece_tjuiagajw_lod4`) (`self.S_Broken_Wooden_Piece_tjuiagajw_lod3`))))

(fn `UserConstructionScript`
  (`parent.UserConstructionScript`))