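; Sheep livestock building Blueprint, a child that relies on its parent class for building behavior.
; On BeginPlay it runs the parent logic, then fills the BuildingParts array with its components, mostly wooden boards and beams plus a few cubes, in a hand-set order.
; The construction script only calls the parent, and the overlap and tick events are disabled stubs.
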(event `self.ReceiveBeginPlay`
  (`parent.ReceiveBeginPlay`)
  (set `self.BuildingParts` (`|MakeArray` (`self.S_Old_Wood_Boards_ricaS_lod3_Var16`) (`self. 2`) (`self. 1`) (`self.3`) (`self.S_Worn_Wooden_Beam_tgmsdc0fa_lod8`) (`self.S_Worn_Wooden_Beam_tgmsdc0fa_lod7`) (`self.S_Worn_Wooden_Beam_tgmsdc0fa_lod6`) (`self.S_Worn_Wooden_Beam_tgmsdc0fa_lod5`) (`self.Cube4`) (`self.Cube1`) (`self.Cube`) (`self.S_Old_Wood_Boards_ricaS_lod3_Var20`) (`self.S_Old_Wood_Boards_ricaS_lod3_Var19`) (`self.S_Old_Wood_Boards_ricaS_lod3_Var25`) (`self.S_Old_Wood_Boards_ricaS_lod3_Var29`) (`self.S_Old_Wood_Boards_ricaS_lod3_Var28`) (`self.S_Old_Wood_Boards_ricaS_lod3_Var27`) (`self.S_Old_Wood_Boards_ricaS_lod3_Var26`) (`self.S_Old_Wood_Boards_ricaS_lod3_Var24`) (`self.S_Old_Wood_Boards_ricaS_lod3_Var21`) (`self.S_Old_Wooden_Beam_wggnei1_lod3_Var8`) (`self.S_Old_Wooden_Beam_wggnei1_lod3_Var7`) (`self.S_Old_Wood_Boards_ricaS_lod3_Var23`) (`self.S_Old_Wood_Boards_ricaS_lod3_Var22`) (`self.Cube2`) (`self.Cube3`) (`self.S_Old_Wood_Boards_ricaS_lod3_Var9`) (`self.S_Old_Wood_Boards_ricaS_lod3_Var11`) (`self.S_Old_Wooden_Beam_wggnei1_lod3_Var1`) (`self.S_Old_Wood_Boards_ricaS_lod3_Var6`) (`self.S_Old_Wood_Boards_ricaS_lod3_Var7`) (`self.S_Old_Wood_Boards_ricaS_lod3_Var10`) (`self.S_Old_Wood_Boards_ricaS_lod3_Var17`) (`self.S_Worn_Wooden_Beam_tgmsdc0fa_lod4`) (`self.S_Old_Wood_Boards_ricaS_lod3_Var8`) (`self.S_Worn_Wooden_Beam_tgmsdc0fa_lod3`) (`self.S_Old_Wooden_Beam_wggnei1_lod3_Var6`) (`self.S_Old_Wood_Boards_ricaS_lod3_Var15`) (`self.S_Old_Wood_Boards_ricaS_lod3_Var14`) (`self.S_Old_Wood_Boards_ricaS_lod3_Var13`) (`self.S_Old_Wooden_Beam_wggnei1_lod3_Var2`) (`self.S_Old_Wood_Boards_ricaS_lod3_Var12`) (`self.S_Old_Wood_Boards_ricaS_lod3_Var18`) (`self.S_Old_Wooden_Beam_wggnei1_lod3_Var4`) (`self.S_Old_Wooden_Beam_wggnei1_lod3_Var3`))))

(fn `UserConstructionScript`
  (`parent.UserConstructionScript`))