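; WellBP is a well building that adds water to the game's resources when it begins play.
; On BeginPlay it runs the parent logic, registers its three cube components as BuildingParts, then raises the Water value on the game mode reference by a fixed amount.
; The construction script only calls the parent, and the overlap and tick events are disabled.
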(event `self.ReceiveBeginPlay`
  (bind _gamemoderef (`self.GamemodeRef`))
  (`parent.ReceiveBeginPlay`)
  (set `self.BuildingParts` (`|MakeArray` (`self.Cube`) (`self.Cube1`) (`self.Cube2`)))
  (set `/Game/BlueprintClasses/RTSBasicGamemode.Water` (+ (`/Game/BlueprintClasses/RTSBasicGamemode.Water` _gamemoderef) 25) _gamemoderef))

(fn `UserConstructionScript`
  (`parent.UserConstructionScript`))