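; Hunter's hut building Blueprint, assembled from modular medieval walls, gables, wooden beams, fences, a campfire, a bench and cubes.
; On BeginPlay it runs the parent logic, then fills the BuildingParts array with these components.
; It adds no other active logic: Tick and overlap events are disabled, and the construction script only calls the parent.
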(event `self.ReceiveBeginPlay`
  (`parent.ReceiveBeginPlay`)
  (set `self.BuildingParts` (`|MakeArray` (`self.S_Medieval_Modular_Door_Wall_udsrdikdw_lod3_Var1`) (`self.S_Medieval_Modular_Wall_uewibagdw_lod3_Var1`) (`self.S_Medieval_Modular_Wall_udsrefrdw_lod3_Var1`) (`self.S_Wooden_Beam_tgnheinfa_lod4`) (`self.S_Wooden_Beam_tgnheinfa_lod5`) (`self.S_Wooden_Beam_tgnheinfa_lod6`) (`self.S_Modular_Fence_ufflaitdw_lod3_Var1`) (`self.S_Wooden_Beam_tgnheinfa_lod7`) (`self.S_Modular_Fence_ufflaitdw_lod3_Var2`) (`self.S_Modular_Fence_ufflaitdw_lod3_Var3`) (`self.S_Campfire_uenpfeifa_lod3_Var1`) (`self.S_Old_Wooden_Bench_uchpfjefa_lod3`) (`self.Cube1`) (`self.S_Medieval_Modular_Corner_Wall_ueoidegdw_lod3_Var1`) (`self.Cube`) (`self.S_Medieval_Modular_Gable_udsreiudw_lod3_Var2`) (`self.S_Medieval_Modular_Corner_Wall_ueoidegdw_lod3_Var2`) (`self.S_Medieval_Modular_Corner_Wall_ueoidegdw_lod3_Var3`) (`self.S_Medieval_Modular_Corner_Wall_ueoidegdw_lod3_Var4`) (`self.S_Medieval_Modular_Wall_udsrefrdw_lod3_Var2`) (`self.S_Medieval_Modular_Gable_udsreiudw_lod3_Var1`))))

(fn `UserConstructionScript`
  (`parent.UserConstructionScript`))