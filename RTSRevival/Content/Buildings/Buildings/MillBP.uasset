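; Mill building Blueprint, a child of a parent building class, built from many separate part components: walls, beams, roofs, a cylinder, a fan assembly and numerous cubes.
; On BeginPlay it runs the parent logic, then fills the BuildingParts array with a hand-ordered list of those components.
; It adds no other behavior: overlap and Tick are disabled, and the construction script only calls the parent.
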(event `self.ReceiveBeginPlay`
  (`parent.ReceiveBeginPlay`)
  (set `self.BuildingParts` (`|MakeArray` (`self.Cylinder`) (`self.BottonWall`) (`self.FrontBeam1`) (`self.FrontBeam2`) (`self.FrontBeam3`) (`self.FrontBeam4`) (`self.FrontBeam5`) (`self.FrontBeam6`) (`self.FrontWall`) (`self.LeftWall`) (`self.RightWall`) (`self.BackWall`) (`self.FrontRoofWall`) (`self.BackRoofWall`) (`self.LeftRoof`) (`self.RightRoof`) (`self.FrontBeam`) (`self.BackBeam`) (`self.Cube14`) (`self.Cube15`) (`self.Cube16`) (`self.Cube9`) (`self.Cube12`) (`self.Cube11`) (`self.Cube10`) (`self.Cube13`) (`self.Cube17`) (`self.Cube21`) (`self.Cube4`) (`self.Cube3`) (`self.Cube2`) (`self.Cube19`) (`self.Cube18`) (`self.Cube8`) (`self.Cube7`) (`self.Cube20`) (`self.Cube6`) (`self.Cube5`) (`self.Cube`) (`self.Cube1`) (`self.FanHolder`) (`self.FanBeam`) (`self.Cube29`) (`self.Cube22`) (`self.Cube27`) (`self.Cube26`) (`self.Cube25`) (`self.Cube24`) (`self.Cube23`) (`self.Cube28`) (`self.Cube30`) (`self.Cube31`) (`self.Cube34`) (`self.Cube33`) (`self.Cube32`) (`self.Cube57`) (`self.Cube56`) (`self.Cube55`) (`self.Cube48`) (`self.Cube53`) (`self.Cube52`) (`self.Cube51`) (`self.Cube50`) (`self.Cube58`) (`self.Cube49`) (`self.Cube60`) (`self.Cube59`) (`self.Cube54`) (`self.Cube38`) (`self.Cube37`) (`self.Cube36`) (`self.Cube41`) (`self.Cube39`) (`self.Cube47`) (`self.Cube46`) (`self.Cube45`) (`self.Cube44`) (`self.Cube43`) (`self.Cube42`) (`self.Cube35`) (`self.Cube40`))))

(fn `UserConstructionScript`
  (`parent.UserConstructionScript`))