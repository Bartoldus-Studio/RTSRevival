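; Farm building Blueprint assembled from medieval modular walls, gables, doors, cubes and props such as barrels, buckets, a wheelbarrow and a campfire.
; BeginPlay runs the parent logic, then fills the BuildingParts array with these components.
; The construction script only calls the parent, and nothing here reads the array.
; Tick and overlap events are disabled placeholders.
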(event `self.ReceiveBeginPlay`
  (`parent.ReceiveBeginPlay`)
  (set `self.BuildingParts` (`|MakeArray` (`self.S_Medieval_Modular_Corner_Wall_udsregzdw_lod3_Var3`) (`self.S_Medieval_Modular_Corner_Wall_udsregzdw_lod3_Var4`) (`self.S_Medieval_Modular_Corner_Wall_udsregzdw_lod3_Var2`) (`self.S_Medieval_Modular_Corner_Wall_udsregzdw_lod3_Var1`) (`self.S_Medieval_Modular_Door_ueoqceudw_lod3_Var1`) (`self.S_Medieval_Modular_Door_Wall_udsrdikdw_lod3_Var1`) (`self.S_Medieval_Modular_Wall_udsrededw_lod3_Var1`) (`self.S_Medieval_Modular_Wall_uewibaydw_lod3_Var1`) (`self.S_Medieval_Modular_Door_ueoqceudw_lod3_Var2`) (`self.S_Medieval_Modular_Wall_uewibaydw_lod3_Var2`) (`self.Cube1`) (`self.Cube`) (`self.S_Medieval_Modular_Gable_udsreiudw_lod3_Var2`) (`self.S_Medieval_Modular_Gable_udsreiudw_lod3_Var1`) (`self.S_Medieval_Modular_Wall_ueojbazdw_lod3_Var1`) (`self.S_Medieval_Modular_Wall_ueojbazdw_lod3_Var2`) (`self.S_Medieval_Modular_Wall_ucsjfhmhx_lod3`) (`self.S_Medieval_Modular_Wall_ucrufcrhx_lod3_Var1`) (`self.S_Half_Timbered_Corner_Wall_ucskaishx_lod3`) (`self.S_Medieval_Modular_Wall_ueoqbdhdw_lod3_Var1`) (`self.S_Medieval_Modular_Gable_udsreiudw_lod3_Var3`) (`self.S_Medieval_Modular_Door_uewibbkdw_lod3_Var1`) (`self.S_Medieval_Modular_Gable_udsreiudw_lod3_Var4`) (`self.S_Medieval_Modular_Wall_ueoqbdhdw_lod3_Var4`) (`self.S_Medieval_Modular_Wall_ueoqbdhdw_lod3_Var3`) (`self.S_Medieval_Modular_Wall_ueoqbdhdw_lod3_Var2`) (`self.S_Half_Timbered_Corner_Wall_ucskaishx_lod4`) (`self.S_Half_Timbered_Corner_Wall_ucskaishx_lod5`) (`self.S_Half_Timbered_Corner_Wall_ucskaishx_lod6`) (`self.S_Medieval_Modular_Wall_ucsjfhmhx_lod4`) (`self.Cube2`) (`self.Cube3`) (`self.S_Wooden_Barrel_tmrveaeda_lod5`) (`self.S_Wooden_Barrel_tmrveaeda_lod4`) (`self.S_Wooden_Wheelbarrow_tmruaaeda_lod3`) (`self.S_Wooden_Wheel_tmrxfdhda_lod3`) (`self.S_Wooden_Barrel_tmrveaeda_lod3`) (`self.S_Tangled_Rope_vhnofbds_lod3_Var1`) (`self.S_Old_Wooden_Bucket_ubupeirfa_lod3`) (`self.S_Campfire_uenpfeifa_lod3_Var1`) (`self.S_Jute_Jug_ueihbhefa_lod3_Var3`) (`self.S_Old_Wooden_Bucket_ubupeirfa_lod5`) (`self.S_Old_Wooden_Bucket_ubupeirfa_lod4`) (`self.S_Jute_Jug_ueihbhefa_lod3_Var1`) (`self.S_Jute_Jug_ueihbhefa_lod3_Var2`) (`self.S_Old_Scythe_tmgqcb2fa_lod3`))))

(fn `UserConstructionScript`
  (`parent.UserConstructionScript`))