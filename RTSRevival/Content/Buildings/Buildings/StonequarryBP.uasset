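; Stone quarry building Blueprint, assembled from prop and primitive components such as pickaxes, wooden beams, a rope, a hook, a pulley, cubes and a cylinder.
; On BeginPlay it runs the parent logic, then fills the BuildingParts array with those components.
; It adds no other active logic: Tick and overlap events are disabled, and the construction script only calls its parent.
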(event `self.ReceiveBeginPlay`
  (`parent.ReceiveBeginPlay`)
  (set `self.BuildingParts` (`|MakeArray` (`self.S_Old_Pickaxe_ucylebxfa_lod4`) (`self.S_Worn_Wooden_Beam_tgnhcaafa_lod4`) (`self.Cylinder`) (`self.Cube4`) (`self.Cube5`) (`self.Cube3`) (`self.Cube2`) (`self.Cube`) (`self.S_Old_Pickaxe_ucylebxfa_lod3`) (`self.S_Tangled_Rope_vhnofbds_lod3_Var1`) (`self.S_Wall_Mounted_Metal_Hook_uiziehxdw_lod3`) (`self.S_Worn_Wooden_Beam_tgnhcaafa_lod3`) (`self.S_Worn_Wooden_Beam_tgnhcaafa_lod5`) (`self.S_Old_Rusty_Pulley_ui2jahm_lod3_Var1`))))

(fn `UserConstructionScript`
  (`parent.UserConstructionScript`))