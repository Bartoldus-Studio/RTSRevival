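; HouseBP is a house building Blueprint assembled from named wall, corner, door wall and roof pieces.
; On BeginPlay it runs the parent logic, then fills the BuildingParts array with these pieces.
; The construction script only calls its parent, and the overlap and tick events are disabled stubs.
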(event `self.ReceiveBeginPlay`
  (`parent.ReceiveBeginPlay`)
  (set `self.BuildingParts` (`|MakeArray` (`self.LeftWall`) (`self.BackLeftCorner`) (`self.BackWall`) (`self.BackRightCorner`) (`self.RightWall`) (`self.FrontRightCorner`) (`self.DoorWall`) (`self.FrontLeftCorner`) (`self.BackRoofWall`) (`self.FrontRoofWall`) (`self.LeftRoof`) (`self.RightRoof`))))

(fn `UserConstructionScript`
  (`parent.UserConstructionScript`))