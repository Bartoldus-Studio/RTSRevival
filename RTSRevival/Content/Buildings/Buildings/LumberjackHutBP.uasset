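; Lumberjack hut building Blueprint, derived from a parent class that it calls on BeginPlay and construction.
; After the parent BeginPlay, it fills the BuildingParts array with its pieces: wood pile, axe, chopping block, firewood, posts and roof.
; The overlap and tick events are disabled, so any further behavior comes from the parent.
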(event `self.ReceiveBeginPlay`
  (`parent.ReceiveBeginPlay`)
  (set `self.BuildingParts` (`|MakeArray` (`self.PileOfWood`) (`self.Axe`) (`self.ChoppingBlock`) (`self.Firewood4`) (`self.Firewood3`) (`self.Firewood2`) (`self.Firewood`) (`self.LeftPost`) (`self.RightPost`) (`self.RoofWood`) (`self.Roof`))))

(fn `UserConstructionScript`
  (`parent.UserConstructionScript`))