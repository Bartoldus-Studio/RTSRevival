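; Tool smithy building Blueprint, assembled from modular medieval walls, gables, roof pieces, wooden beams and blacksmith props such as an anvil, hammer and tongs.
; On BeginPlay it runs the parent logic, then fills the BuildingParts array with a hand-ordered list of its components.
; The array is not used in this graph, and the construction script only calls the parent.
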(event `self.ReceiveBeginPlay`
  (`parent.ReceiveBeginPlay`)
  (set `self.BuildingParts` (`|MakeArray` (`self.S_Medieval_Modular_Wall_ucsibafhx_lod3_Var2`) (`self.S_Medieval_Modular_Corner_Wall_uebrabtdw_lod3_Var4`) (`self.S_Medieval_Modular_Gable_uebrcgcdw_lod3_Var2`) (`self.S_Modular_Wooden_Roof_wkupbctdw_lod3_Var2`) (`self.S_Modular_Wooden_Roof_wkupbctdw_lod3_Var3`) (`self.S_Wooden_Beam_tgnheinfa_lod4`) (`self.S_Wooden_Beam_tgnheinfa_lod6`) (`self.S_Wooden_Beam_tgnheinfa_lod5`) (`self.S_Wooden_Beam_tgnheinfa_lod7`) (`self.S_Modular_Wooden_Roof_wkupbctdw_lod3_Var4`) (`self.Cube3`) (`self.Cube2`) (`self.Cube4`) (`self.S_Medieval_Modular_Corner_Wall_uebrabtdw_lod3_Var2`) (`self.S_Medieval_Modular_Corner_Wall_uebrabtdw_lod3_Var3`) (`self.S_Blacksmith_Tongs_udmjddsqx_lod3`) (`self.S_Medieval_Modular_Door_Wall_uebmci3dw_lod3_Var1`) (`self.S_Old_Hammer_uc1mfe1fa_lod3`) (`self.S_Medieval_Modular_Wall_uebmdapdw_lod3_Var1`) (`self.S_Medieval_Modular_Gable_uebrcgcdw_lod3_Var1`) (`self.S_Medieval_Modular_Wall_ucsibafhx_lod3_Var1`) (`self.S_Medieval_Modular_Corner_Wall_uebrabtdw_lod3_Var1`) (`self.S_Blacksmith_Anvil_tmgtaedfa_lod3`))))

(fn `UserConstructionScript`
  (`parent.UserConstructionScript`))