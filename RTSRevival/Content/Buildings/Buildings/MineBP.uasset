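; Mine building, a child of a shared building Blueprint, that produces Metal for the player.
; On BeginPlay it runs the parent setup, then registers its tunnel, tool and box meshes as BuildingParts and sets its ProductionDay.
; Its resource usage override calls the parent, then increments Metal on the game mode by one.
; Day handling is left entirely to the parent class.
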(event `self.ReceiveBeginPlay`
  (`parent.ReceiveBeginPlay`)
  (set `self.BuildingParts` (`|MakeArray` (`self.S_Wooden_Wheelbarrow_tmruaaeda_lod3`) (`self.S_Rusty_Shovel_uddjeelqx_lod3`) (`self.S_Old_Pickaxe_ucylebxfa_lod5`) (`self.S_Old_Pickaxe_ucylebxfa_lod4`) (`self.S_Old_Pickaxe_ucylebxfa_lod3`) (`self.Cube2`) (`self.Cube1`) (`self.Cube`) (`self.S_Modular_Mine_Tunnel_Start-end_wcbpdfsdw_lod3_Var1`) (`self.Box_836ABAFE`)))
  (set `self.ProductionDay` 3))

(fn `ManageNewDay`
  (`parent.ManageNewDay`))

(fn `ManageRessourceUsage`
  (`parent.ManageRessourceUsage`)
  (`/Engine/EditorBlueprintResources/StandardMacros.IncrementInt` (`/Game/BlueprintClasses/RTSBasicGamemode.Metal` (`self.GamemodeRef`))))

(fn `UserConstructionScript`
  (`parent.UserConstructionScript`))