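; BakeryBP is a bakery building Blueprint assembled from medieval modular walls, doors, gables, half-timbered corners, cubes and bread props.
; On BeginPlay it calls the parent, then fills the BuildingParts array with these components.
; The file does not use that array further, and the construction script only calls its parent.
; Overlap and Tick events are disabled stubs.
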(event `self.ReceiveBeginPlay`
  (`parent.ReceiveBeginPlay`)
  (set `self.BuildingParts` (`|MakeArray` (`self.S_Half_Timbered_Corner_Wall_ucskaishx_lod4`) (`self.S_Medieval_Modular_Door_ueojadodw_lod3_Var1`) (`self.S_Half_Timbered_Corner_Wall_ucskaishx_lod3`) (`self.S_Medieval_Modular_Wall_ueoqbdhdw_lod3_Var1`) (`self.S_Medieval_Modular_Wall_ueoqbdhdw_lod3_Var2`) (`self.S_Medieval_Modular_Wall_ueojbazdw_lod3_Var1`) (`self.Cube`) (`self.Cube1`) (`self.Cube2`) (`self.S_Medieval_Modular_Gable_udsreiudw_lod3_Var2`) (`self.S_Medieval_Modular_Gable_udsreiudw_lod3_Var1`) (`self.S_Medieval_Modular_Door_uewibbkdw_lod3_Var1`) (`self.S_Half_Timbered_Corner_Wall_ucskaishx_lod6`) (`self.S_Half_Timbered_Corner_Wall_ucskaishx_lod5`) (`self.Cube3`) (`self.Cube4`) (`self.Cube5`) (`self.S_Bread_Roll_thqsfdepa_lod4`) (`self.S_Bread_Roll_thqsfdepa_lod3`) (`self.S_Black_Bread_te0kbikpa_lod3_Var1`))))

(fn `UserConstructionScript`
  (`parent.UserConstructionScript`))