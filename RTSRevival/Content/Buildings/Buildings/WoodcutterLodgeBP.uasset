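; Woodcutter lodge building Blueprint, assembled from named parts such as posts, roof pieces, a chopping block, axes and cubes.
; On BeginPlay it runs the parent logic, then fills the BuildingParts array with those parts.
; It adds no other logic: overlap and tick events are disabled, and the construction script only calls the parent.
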(event `self.ReceiveBeginPlay`
  (`parent.ReceiveBeginPlay`)
  (set `self.BuildingParts` (`|MakeArray` (`self.FrontPost`) (`self.BackPost`) (`self.RoofBeam`) (`self. RightRoof`) (`self.LeftRoof`) (`self.ChoppingBlock`) (`self.Axe`) (`self.Axe1`) (`self.Cube`) (`self.Cube1`) (`self.Cube2`) (`self.Cube3`) (`self.Cube4`) (`self.Cube5`))))

(fn `UserConstructionScript`
  (`parent.UserConstructionScript`))