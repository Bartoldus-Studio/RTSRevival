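; Butcher house building Blueprint, assembled from cube pieces and wall-mounted metal hook meshes.
; On BeginPlay it runs the parent logic first, then fills the BuildingParts array with those components.
; The construction script only calls the parent, and the overlap and Tick events are disabled stubs, so any other behavior comes from the parent class.
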(event `self.ReceiveBeginPlay`
  (`parent.ReceiveBeginPlay`)
  (set `self.BuildingParts` (`|MakeArray` (`self.Cube`) (`self.Cube1`) (`self.Cube2`) (`self.Cube3`) (`self.Cube4`) (`self.Cube5`) (`self.Cube6`) (`self.Cube7`) (`self.Cube8`) (`self.Cube9`) (`self.Cube10`) (`self.Cube11`) (`self.Cube12`) (`self.Cube13`) (`self.Cube14`) (`self.Cube15`) (`self.Cube16`) (`self.Cube17`) (`self.Cube18`) (`self.Cube19`) (`self.Cube20`) (`self.Cube21`) (`self.S_Wall_Mounted_Metal_Hook_uiziehxdw_lod3`) (`self.S_Wall_Mounted_Metal_Hook_uiziehxdw_lod4`) (`self.S_Wall_Mounted_Metal_Hook_uiziehxdw_lod6`) (`self.S_Wall_Mounted_Metal_Hook_uiziehxdw_lod7`) (`self.S_Wall_Mounted_Metal_Hook_uiziehxdw_lod5`))))

(fn `UserConstructionScript`
  (`parent.UserConstructionScript`))