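; Cow livestock building, a child Blueprint assembled from modular medieval walls, doors, gables and fences, plus cubes and props such as buckets and a wheelbarrow.
; On BeginPlay it runs the parent logic, then fills the BuildingParts array with these components in a fixed order.
; It has no other logic of its own: overlap and tick are disabled, and the construction script only calls the parent.
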(event `self.ReceiveBeginPlay`
  (`parent.ReceiveBeginPlay`)
  (set `self.BuildingParts` (`|MakeArray` (`self.S_Modular_Fence_ufflaitdw_lod3_Var17`) (`self.S_Modular_Fence_ufflaitdw_lod3_Var1`) (`self.S_Medieval_Modular_Door_ueoqceudw_lod3_Var1`) (`self.S_Medieval_Modular_Corner_Wall_udsregzdw_lod3_Var1`) (`self.S_Medieval_Modular_Corner_Wall_udsregzdw_lod3_Var2`) (`self.S_Medieval_Modular_Corner_Wall_udsregzdw_lod3_Var3`) (`self.S_Medieval_Modular_Door_ueoqceudw_lod3_Var2`) (`self.S_Medieval_Modular_Wall_udsreafdw_lod3_Var1`) (`self.S_Medieval_Modular_Corner_Wall_udsregzdw_lod3_Var4`) (`self.S_Medieval_Modular_Wall_udsreafdw_lod3_Var2`) (`self.S_Medieval_Modular_Wall_udsreafdw_lod3_Var3`) (`self.S_Medieval_Modular_Wall_udsreafdw_lod3_Var4`) (`self.S_Medieval_Modular_Gable_ucrtdgdhx_lod3`) (`self.S_Medieval_Modular_Gable_ucrtdgdhx_lod4`) (`self.S_Modular_Fence_ufflaitdw_lod3_Var13`) (`self.S_Modular_Fence_ufflaitdw_lod3_Var16`) (`self.S_Modular_Fence_ufflaitdw_lod3_Var3`) (`self.S_Modular_Fence_ufflaitdw_lod3_Var2`) (`self.S_Modular_Fence_ufflaitdw_lod3_Var4`) (`self.S_Modular_Fence_ufflaitdw_lod3_Var12`) (`self.S_Modular_Fence_ufflaitdw_lod3_Var5`) (`self.S_Modular_Fence_ufflaitdw_lod3_Var6`) (`self.S_Modular_Fence_ufflaitdw_lod3_Var7`) (`self.S_Modular_Fence_ufflaitdw_lod3_Var8`) (`self.S_Modular_Fence_ufflaitdw_lod3_Var9`) (`self.S_Modular_Fence_ufflaitdw_lod3_Var10`) (`self.S_Modular_Fence_ufflaitdw_lod3_Var11`) (`self.Cube`) (`self.Cube1`) (`self.S_Old_Wooden_Bucket_ubupeirfa_lod6`) (`self.S_Old_Wooden_Bucket_ubupeirfa_lod3`) (`self.S_Wooden_Wheelbarrow_tmruaaeda_lod3`) (`self.S_Old_Wooden_Bucket_ubupeirfa_lod5`))))

(fn `UserConstructionScript`
  (`parent.UserConstructionScript`))