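; LoggingCampBP is a logging camp building that adds one wood to the game mode's resources each new day.
; On BeginPlay it runs the parent logic, then fills BuildingParts with its campfire, beam, posts, roof halves and cube components.
; Its ManageNewDay override calls the parent version before incrementing Wood through GamemodeRef, leaving all other behavior to the parent class.
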(event `self.ReceiveBeginPlay`
  (`parent.ReceiveBeginPlay`)
  (set `self.BuildingParts` (`|MakeArray` (`self.Campfire`) (`self.RoofBeam`) (`self.BackPost`) (`self.FrontPost`) (`self. RightRoof`) (`self.LeftRoof`) (`self.Cube`) (`self.Cube1`) (`self.Cube2`) (`self.Cube3`) (`self.Cube4`) (`self.Cube5`) (`self.Cube6`) (`self.Cube7`) (`self.Cube8`) (`self.Cube9`) (`self.Cube10`) (`self.Cube11`) (`self.Cube13`) (`self.Cube14`))))

(fn `ManageNewDay`
  (`parent.ManageNewDay`)
  (`/Engine/EditorBlueprintResources/StandardMacros.IncrementInt` (`/Game/BlueprintClasses/RTSBasicGamemode.Wood` (`self.GamemodeRef`))))

(fn `UserConstructionScript`
  (`parent.UserConstructionScript`))