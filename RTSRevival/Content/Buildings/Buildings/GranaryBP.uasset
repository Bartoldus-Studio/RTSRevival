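; Granary building Blueprint, assembled from modular medieval mesh parts such as walls, corners, doors and gables, plus several cube components.
; On BeginPlay it runs the parent logic, then fills the BuildingParts array with a fixed list of those components.
; Nothing in this file reads the array, and the construction script only calls its parent.
; Tick and overlap events are disabled stubs.
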(event `self.ReceiveBeginPlay`
  (`parent.ReceiveBeginPlay`)
  (set `self.BuildingParts` (`|MakeArray` (`self.S_Half_Timbered_Corner_Wall_ucskaishx_lod4`) (`self.S_Half_Timbered_Corner_Wall_ucskaishx_lod3`) (`self.S_Medieval_Modular_Wall_ucsjfhmhx_lod3`) (`self.S_Medieval_Modular_Wall_ucrufcrhx_lod3_Var1`) (`self.S_Medieval_Modular_Wall_ucsjfhmhx_lod5`) (`self.S_Medieval_Modular_Door_uewibbkdw_lod3_Var1`) (`self.S_Half_Timbered_Corner_Wall_ucskaishx_lod6`) (`self.S_Medieval_Modular_Wall_ucsjfhmhx_lod4`) (`self.S_Half_Timbered_Corner_Wall_ucskaishx_lod5`) (`self.S_Medieval_Modular_Door_Wall_udsrdikdw_lod3_Var1`) (`self.S_Medieval_Modular_Corner_Wall_udsregzdw_lod3_Var1`) (`self.S_Medieval_Modular_Corner_Wall_udsregzdw_lod3_Var2`) (`self.S_Medieval_Modular_Wall_uewibaydw_lod3_Var1`) (`self.S_Medieval_Modular_Corner_Wall_udsregzdw_lod3_Var3`) (`self.S_Medieval_Modular_Wall_uewibaydw_lod3_Var2`) (`self.S_Medieval_Modular_Wall_uewibaydw_lod3_Var3`) (`self.S_Medieval_Modular_Corner_Wall_udsregzdw_lod3_Var4`) (`self.S_Medieval_Modular_Gable_udsreiudw_lod3_Var1`) (`self.S_Medieval_Modular_Gable_udsreiudw_lod3_Var2`) (`self.Cube`) (`self.Cube1`) (`self.Cube8`) (`self.Cube17`) (`self.Cube18`))))

(fn `UserConstructionScript`
  (`parent.UserConstructionScript`))