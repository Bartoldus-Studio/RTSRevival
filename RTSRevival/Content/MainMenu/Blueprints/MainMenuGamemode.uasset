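; Main menu game mode for an RTS that shows the main menu widget on BeginPlay and handles menu navigation, quitting and starting the game.
; It passes itself to the MainMenuGUI and StartGameMenu widgets, creates each on demand and swaps them in and out of the viewport.
; Preset resource changes are written to the RTSGameInstance, and starting the game opens TestMap.
; The OptionsMenu event is an empty stub.
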(event `self.ReceiveBeginPlay`
  (bind _returnvalue (`|CreateWidget` "/Game/MainMenu/MainMenuGUI.MainMenuGUI_C" (`GameplayStatics.GetPlayerController` 0) self))
  (bind _output_get (set `self.MainMenuGUIRef` _returnvalue))
  (`UserWidget.AddToViewport` _output_get 0))

(event `QuitApplication`
  (`KismetSystemLibrary.QuitGame` (`GameplayStatics.GetPlayerController` 0) "Quit"))

(event `StartGameMenu`
  (`Widget.RemoveFromParent` (`self.MainMenuGUIRef`))
  (`/Engine/EditorBlueprintResources/StandardMacros.IsValid` (`self.StartGameGUIRef`)
    (:`Is Valid`
      _)
    (:`Is Not Valid`
      (bind _returnvalue (`|CreateWidget` "/Game/MainMenu/StartGameMenu.StartGameMenu_C" (`GameplayStatics.GetPlayerController` 0) self))
      (set `self.StartGameGUIRef` _returnvalue)))
  (`UserWidget.AddToViewport` (`self.StartGameGUIRef`) 0))

(event `OptionsMenu`)

(event `BackToMainMenu`
  (params (CurrentOpenWidget :type "UserWidget Object Reference"))
  (bind _mainmenuguiref (`self.MainMenuGUIRef`))
  (`Widget.RemoveFromParent` CurrentOpenWidget)
  (`/Engine/EditorBlueprintResources/StandardMacros.IsValid` _mainmenuguiref
    (:`Is Valid`
      _)
    (:`Is Not Valid`
      (bind _returnvalue (`|CreateWidget` "/Game/MainMenu/MainMenuGUI.MainMenuGUI_C" (`GameplayStatics.GetPlayerController` 0) self))
      (set `self.MainMenuGUIRef` _returnvalue)))
  (`UserWidget.AddToViewport` _mainmenuguiref 0))

(event `StartGame`
  (`GameplayStatics.OpenLevel` "TestMap"))

(event `PresetDataChanged`
  (params (Wood :type Integer) (Stone :type Integer) (Metal :type Integer) (Bread :type Integer) (Berries :type Integer) (Meat :type Integer))
  (bind _asrtsgame_instance (cast `/Game/BlueprintClasses/RTSGameInstance` (`GameplayStatics.GetGameInstance`)))
  (`/Game/BlueprintClasses/RTSGameInstance.SetGamePresets` _asrtsgame_instance Wood Stone Metal Bread Berries Meat))

(fn `UserConstructionScript`)